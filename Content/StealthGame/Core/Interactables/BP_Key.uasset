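; BP_Key is a collectible key pickup for the stealth game.
; When the player character overlaps its box collision, it increments that character's KeyCount, destroys itself and calls ShowKeyWidget on player character 0.
; BeginPlay creates a key widget without storing or displaying it, and debug prints trace the pickup.
; The Show/HideKeyWidget event holds only an unconnected FlipFlop.
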(event `self.ReceiveBeginPlay`
  (`|ExecutionSequence`
    (:`then_0`
      (`|CreateWidget` "/Game/StealthGame/MaterialLibrary/Widgets/W_KeyWidget.W_KeyWidget_C"))
    (:`then_1`
      (`KismetSystemLibrary.PrintString` "This Key Exists!" true true (struct :`R` 0.989389 :`G` 0.130208 :`B` 1.0 :`A` 1.0)))))

(event `self.Box Collision.OnComponentBeginOverlap`
  (params (OverlappedComponent :type "PrimitiveComponent Object Reference") (OtherActor :type "Actor Object Reference") (OtherComp :type "PrimitiveComponent Object Reference") (OtherBodyIndex :type Integer) (bFromSweep :type Boolean) (SweepResult :type "HitResult Structure (by ref)"))
  (bind _asbp_third_person_character_custom (cast `/Game/StealthGame/Core/Characters/PlayerCharacter/BP_ThirdPersonCharacterCustom` OtherActor)
    (:`then`
      (`KismetSystemLibrary.PrintString` "Key has been Overlapped by Player" true true (struct :`G` 0.66 :`B` 1.0 :`A` 1.0) 5.0)
      (bind _key_count (`/Game/StealthGame/Core/Characters/PlayerCharacter/BP_ThirdPersonCharacterCustom.Key Count` _asbp_third_person_character_custom))
      (set `/Game/StealthGame/Core/Characters/PlayerCharacter/BP_ThirdPersonCharacterCustom.Key Count` (+ _key_count 1) _asbp_third_person_character_custom) ; Set Key Count
      (`KismetSystemLibrary.PrintString` (`KismetStringLibrary.Concat_StrStr` "The Player has " (`KismetStringLibrary.Conv_IntToString` _key_count) " key(s)."))
      (`|ExecutionSequence`
        (:`then_0`
          (`self.K2_DestroyActor`) ; Destroy this key
        )
        (:`then_1`
          (bind _asbp_third_person_character_custom_2 (cast `/Game/StealthGame/Core/Characters/PlayerCharacter/BP_ThirdPersonCharacterCustom` (`GameplayStatics.GetPlayerCharacter` 0)))
          (`/Game/StealthGame/Core/Characters/PlayerCharacter/BP_ThirdPersonCharacterCustom.Show Key Widget` _asbp_third_person_character_custom_2))))
    (:`CastFailed`
      (`KismetSystemLibrary.PrintString` "Key Player Cast Failed" true true (struct :`R` 0.875 :`B` 0.029306 :`A` 1.0)))))

(event `Show/Hide Key Widget`
  (`/Engine/EditorBlueprintResources/StandardMacros.FlipFlop`))

(fn `UserConstructionScript`)